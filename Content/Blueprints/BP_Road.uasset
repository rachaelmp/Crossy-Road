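; BP_Road is a road tile that spawns vehicle traffic and removes itself some time after the chicken reaches it.
; On BeginPlay it randomly picks one traffic direction and starts a looping timer with a randomized interval, rolled once.
; Each tick of that timer spawns a BP_Vehicle at the left spawn point or right despawn zone, rotated to match.
; A BP_Chicken entering TriggerZone gives the road a limited lifespan; vehicle lifespan calls are disconnected.
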(event `self.ReceiveBeginPlay`
  (set `self.LeftOrRight` (`KismetMathLibrary.RandomBool`))
  (set `self.Start` (`SceneComponent.K2_GetComponentLocation` (`self.MovingObjectSpawnPointLeft`)))
  (set `self.End` (`SceneComponent.K2_GetComponentLocation` (`self.MovingObjectDespawnZoneRight`)))
  (`KismetSystemLibrary.K2_SetTimerDelegate` (delegate `SpawnVehicles`) (`KismetMathLibrary.RandomFloatInRange` 3.0 5.0) true))

(event `SpawnVehicles`
  (if (`self.LeftOrRight`)
    (bind _returnvalue (`|SpawnActorFromClass` "/Game/Blueprints/BP_Vehicle.BP_Vehicle_C" (`KismetMathLibrary.MakeTransform` (`self.Start`) (struct :`Yaw` 90.0)) "Undefined" "OverrideRootScale" null null))
    (else
      (bind _returnvalue_2 (`|SpawnActorFromClass` "/Game/Blueprints/BP_Vehicle.BP_Vehicle_C" (`KismetMathLibrary.MakeTransform` (`self.End`) (struct :`Yaw` -90.0)) "Undefined" "OverrideRootScale" null null)))))

(event `self.TriggerZone.OnComponentBeginOverlap`
  (params (OverlappedComponent :type "PrimitiveComponent Object Reference") (OtherActor :type "Actor Object Reference") (OtherComp :type "PrimitiveComponent Object Reference") (OtherBodyIndex :type Integer) (bFromSweep :type Boolean) (SweepResult :type "HitResult Structure (by ref)"))
  (cast `/Game/Blueprints/BP_Chicken` OtherActor)
  (`self.SetLifeSpan` 10.0))

(fn `UserConstructionScript`)