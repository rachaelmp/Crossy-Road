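; BP_VehicleSpawner spawns BP_Vehicle actors for a lane, creating one when play begins.
; It picks the lane's left or right spawn point from the lane's FromLeftOrRight setting and spawns the vehicle at that world location.
; Each spawn is stored as NewestVehicle and receives a reference back to the spawner.
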(event `self.ReceiveBeginPlay`
  (`self.SpawnInitialVehicles`))

(fn `SpawnInitialVehicles`
  (`self.SpawnVehicleAtPoint`))

(fn `SpawnVehicle`
  (params (SpawnLocation :type "Vector Structure"))
  (bind _returnvalue (`|SpawnActorFromClass` "/Game/Blueprints/BP_Vehicle.BP_Vehicle_C" (`KismetMathLibrary.MakeTransform` SpawnLocation) "Undefined" "OverrideRootScale" null null))
  (bind _output_get (set `self.NewestVehicle` _returnvalue))
  (set `/Game/Blueprints/BP_Vehicle.VehicleSpawner` self _output_get))

(fn `SpawnVehicleAtPoint`
  (bind _lane (`self.Lane`))
  (`self.SpawnVehicle` (`SceneComponent.K2_GetComponentLocation` (select `int` (`/Game/Blueprints/BP_Road.fromLeftOrRight` _lane) :`0` (`/Game/Blueprints/BP_Road.MovingObjectSpawnPointLeft` _lane) :`1` (`/Game/Blueprints/BP_Road.MovingObjectSpawnPointRight` _lane)))))

(fn `UserConstructionScript`)