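; BP_Chicken is a player-controllable chicken that moves on forward and right axis inputs and turns its mesh to face the travel direction.
; Axis events add movement input scaled by MaxSpeed, which Tick consumes as a swept local offset without delta-time scaling.
; Four DoOnce gates, one per direction, each set a fixed world rotation and reset the other three.
; The rotation lerps use full alpha, so turns snap instantly.
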(event `InputAxis|MoveForward`
  (params (AxisValue :type "Float (single-precision)"))
  (bind _chickenmesh (`self.ChickenMesh`))
  (bind _chickenmesh_2 (`self.ChickenMesh`))
  (bind _chickenmesh_3 (`self.ChickenMesh`))
  (bind _chickenmesh_4 (`self.ChickenMesh`))
  (`self.AddMovementInput` (`self.GetActorForwardVector`) (* AxisValue (`self.MaxSpeed`)))
  (if (< AxisValue 0.0)
    (`/Engine/EditorBlueprintResources/StandardMacros.DoOnce` false :!label _label
      (:`Completed`
        (`SceneComponent.K2_SetWorldRotation` _chickenmesh_2 (`KismetMathLibrary.RLerp` (`SceneComponent.K2_GetComponentRotation` _chickenmesh_2) (struct :`Roll` 90.0) 1.0 true) false false)
        (`|ExecutionSequence`
          (:`then_0`
            (goto _label_2 :!via `Reset`))
          (:`then_1`
            (goto _label_3 :!via `Reset`))
          (:`then_2`
            (goto _label_4 :!via `Reset`)))))
    (elif (> AxisValue 0.0)
      (`/Engine/EditorBlueprintResources/StandardMacros.DoOnce` false :!label _label_2
        (:`Completed`
          (`SceneComponent.K2_SetWorldRotation` _chickenmesh (`KismetMathLibrary.RLerp` (`SceneComponent.K2_GetComponentRotation` _chickenmesh) (struct :`Yaw` 180.0 :`Roll` 90.0) 1.0 true) false false)
          (`|ExecutionSequence`
            (:`then_0`
              (goto _label :!via `Reset`))
            (:`then_1`
              (goto _label_3 :!via `Reset`))
            (:`then_2`
              (goto _label_4 :!via `Reset`))))))))

(event `InputAxis|MoveRight`
  (params (AxisValue :type "Float (single-precision)"))
  (bind _chickenmesh (`self.ChickenMesh`))
  (bind _chickenmesh_2 (`self.ChickenMesh`))
  (`self.AddMovementInput` (`self.GetActorRightVector`) (* AxisValue (`self.MaxSpeed`)))
  (if (< AxisValue 0.0)
    (`/Engine/EditorBlueprintResources/StandardMacros.DoOnce` false :!label _label_3
      (:`Completed`
        (`SceneComponent.K2_SetWorldRotation` _chickenmesh (`KismetMathLibrary.RLerp` (`SceneComponent.K2_GetComponentRotation` _chickenmesh) (struct :`Yaw` 90.0 :`Roll` 90.0) 1.0 true) false false)
        (`|ExecutionSequence`
          (:`then_0`
            (goto _label :!via `Reset`))
          (:`then_1`
            (goto _label_2 :!via `Reset`))
          (:`then_2`
            (goto _label_4 :!via `Reset`)))))
    (elif (> AxisValue 0.0)
      (`/Engine/EditorBlueprintResources/StandardMacros.DoOnce` false :!label _label_4
        (:`Completed`
          (`SceneComponent.K2_SetWorldRotation` _chickenmesh_2 (`KismetMathLibrary.RLerp` (`SceneComponent.K2_GetComponentRotation` _chickenmesh_2) (struct :`Yaw` -90.0 :`Roll` 90.0) 1.0 true) false false)
          (`|ExecutionSequence`
            (:`then_0`
              (goto _label :!via `Reset`))
            (:`then_1`
              (goto _label_2 :!via `Reset`))
            (:`then_2`
              (goto _label_3 :!via `Reset`))))))))

(event `self.ReceiveTick`
  (params (DeltaSeconds :type "Float (single-precision)"))
  (bind _returnvalue (`self.ConsumeMovementInputVector`))
  (`self.K2_AddActorLocalOffset` _returnvalue true))

(fn `UserConstructionScript`)