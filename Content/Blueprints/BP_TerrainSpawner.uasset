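; Terrain spawner that lays out randomized lanes of road, river, train track and grass variants, suggesting a Crossy Road-style crossing game.
; On BeginPlay it spawns a fixed run of evenly spaced lanes along X from LaneMesh's location, keeping the first few as plain grass and randomizing the rest.
; SpawnTerrain repeats the random pick to spawn one lane at a given point, but nothing in this Blueprint calls it.
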(event `self.ReceiveBeginPlay`
  (bind (_returnvalue_x _returnvalue_y _returnvalue_z) (`KismetMathLibrary.BreakVector` (`SceneComponent.K2_GetComponentLocation` (`self.LaneMesh`))))
  (for _index (range 41)
    (set `self.SpawnLocation` (`KismetMathLibrary.MakeVector` (`KismetMathLibrary.Conv_IntToDouble` (+ (* _index 80) (`KismetMathLibrary.FTrunc` _returnvalue_x))) _returnvalue_y _returnvalue_z))
    (if (`KismetMathLibrary.InRange_IntInt` _index 0 2)
      (`|SpawnActorFromClass` "/Game/Blueprints/BP_Grass.BP_Grass_C" (`KismetMathLibrary.MakeTransform` (`self.SpawnLocation`)) "Undefined" "OverrideRootScale" null null)
      (else
        (switch `int` (`KismetMathLibrary.RandomInteger` 6)
          (:`0`
            (`|SpawnActorFromClass` "/Game/Blueprints/BP_Road.BP_Road_C" (`KismetMathLibrary.MakeTransform` (`self.SpawnLocation`)) "Undefined" "OverrideRootScale" null null))
          (:`1`
            (`|SpawnActorFromClass` "/Game/Blueprints/BP_River.BP_River_C" (`KismetMathLibrary.MakeTransform` (`self.SpawnLocation`)) "Undefined" "OverrideRootScale" null null))
          (:`2`
            (`|SpawnActorFromClass` "/Game/Blueprints/BP_Grass.BP_Grass_C" (`KismetMathLibrary.MakeTransform` (`self.SpawnLocation`)) "Undefined" "OverrideRootScale" null null))
          (:`3`
            (`|SpawnActorFromClass` "/Game/Blueprints/BP_TrainTrack.BP_TrainTrack_C" (`KismetMathLibrary.MakeTransform` (`self.SpawnLocation`)) "Undefined" "OverrideRootScale" null null))
          (:`4`
            (`|SpawnActorFromClass` "/Game/Blueprints/BP_Grass_2.BP_Grass_2_C" (`KismetMathLibrary.MakeTransform` (`self.SpawnLocation`)) "Undefined" "OverrideRootScale" null null))
          (:`5`
            (`|SpawnActorFromClass` "/Game/Blueprints/BP_Grass_3.BP_Grass_3_C" (`KismetMathLibrary.MakeTransform` (`self.SpawnLocation`)) "Undefined" "OverrideRootScale" null null)))))))

(fn `SpawnTerrain`
  (params (Spawnpoint :type "Vector Structure"))
  (switch `int` (`KismetMathLibrary.RandomInteger` 6)
    (:`0`
      (`|SpawnActorFromClass` "/Game/Blueprints/BP_Road.BP_Road_C" (`KismetMathLibrary.MakeTransform` Spawnpoint) "Undefined" "OverrideRootScale" null null))
    (:`1`
      (`|SpawnActorFromClass` "/Game/Blueprints/BP_River.BP_River_C" (`KismetMathLibrary.MakeTransform` Spawnpoint) "Undefined" "OverrideRootScale" null null))
    (:`2`
      (`|SpawnActorFromClass` "/Game/Blueprints/BP_Grass.BP_Grass_C" (`KismetMathLibrary.MakeTransform` Spawnpoint) "Undefined" "OverrideRootScale" null null))
    (:`3`
      (`|SpawnActorFromClass` "/Game/Blueprints/BP_TrainTrack.BP_TrainTrack_C" (`KismetMathLibrary.MakeTransform` Spawnpoint) "Undefined" "OverrideRootScale" null null))
    (:`4`
      (`|SpawnActorFromClass` "/Game/Blueprints/BP_Grass_2.BP_Grass_2_C" (`KismetMathLibrary.MakeTransform` Spawnpoint) "Undefined" "OverrideRootScale" null null))
    (:`5`
      (`|SpawnActorFromClass` "/Game/Blueprints/BP_Grass_3.BP_Grass_3_C" (`KismetMathLibrary.MakeTransform` Spawnpoint) "Undefined" "OverrideRootScale" null null))))

(fn `UserConstructionScript`)